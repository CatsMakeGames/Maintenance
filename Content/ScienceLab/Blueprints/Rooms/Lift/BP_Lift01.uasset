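; BP_Lift01 is a lift prop for the ScienceLab rooms, with a body and two sliding doors posed at construction time.
; The construction script offsets the right and left doors in opposite directions along relative X by DoorPosition, then applies one shared Material to both doors and the lift body.
; It has no runtime logic, as the event graph holds only disabled placeholder events.
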(event EventBeginPlay)

(event Collision|EventActorBeginOverlap
  (params (OtherActor :type Actor%20Object%20Reference)))

(event EventTick
  (params (DeltaSeconds :type Float%20%28single-precision%29)))

(fn ConstructionScript
  (bind _leftdoor (Variables|Default|GetLeftDoor))
  (bind _doorposition (Variables|Default|GetDoorPosition))
  ;[1 1 1] Movement
  (Transformation|AddRelativeLocation (Variables|Default|GetRightDoor) (Math|Vector|MakeVector _doorposition 0.0 0.0) false false)
  (Transformation|AddRelativeLocation _leftdoor (Math|Vector|MakeVector (* _doorposition -1.0) 0.0 0.0) false false)
  ;[1 1 1] Material
  (Rendering|Material|SetMaterial _leftdoor 0 (Variables|Default|GetMaterial)))