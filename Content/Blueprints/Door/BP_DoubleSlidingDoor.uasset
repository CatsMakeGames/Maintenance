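; Double sliding door actor with two panels that slide apart symmetrically along their local Y axis.
; The construction script sets the panels open or closed from IsOpen.
; Open plays a slide sound and plays or reverses the timeline according to IsOpen, which this file never updates.
; The timeline's Movement track drives LeftDoor's offset, negated for RightDoor, between the closed and open positions.
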(event EventBeginPlay)

(event Collision|EventActorBeginOverlap
  (params (OtherActor :type Actor%20Object%20Reference)))

(event EventTick
  (params (DeltaSeconds :type Float%20%28single-precision%29)))

(fn ConstructionScript
  (bind _leftdoor (Variables|Default|GetLeftDoor))
  (bind _rightdoor (Variables|Default|GetRightDoor))
  (if (Variables|Default|GetIsOpen)
    (Transformation|SetRelativeLocation _leftdoor "0,140.000000, 0" false false)
    (Transformation|SetRelativeLocation _rightdoor "0,-140.000000, 0" false false)
    (else
      (Transformation|SetRelativeLocation _leftdoor "0,48.000000, 0" false false)
      (Transformation|SetRelativeLocation _rightdoor "0,-48.000000, 0" false false))))

(fn Open
  (bind _open_timeline (Variables|Default|GetOpen_TimeLine))
  (Audio|PlaySoundatLocation "/Game/Sounds/bms/doors/doorslide_opening1_Cue1.doorslide_opening1_Cue1" (Transformation|GetActorLocation) "0, 0, 0" 1.0 1.0 0.0 0 0 0)
  (if (Variables|Default|GetIsOpen)
    (Utilities|String|Reverse _open_timeline)
    (else
      (Audio|Components|Audio|Play _open_timeline))))