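; Interactable door that swings its mesh open or shut when toggled, with sounds for movement end, locked and unlocked states.
; Toggle plays or reverses a Movement timeline that drives yaw up to 90 degrees, with Reverse choosing swing direction and construction script setting play rate.
; On finish it stops the DefaultMove loop, flips Open and fires OnFinishedMovement.
; UseItem defers to the parent, then prints the item's name.
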(event EventBeginPlay)

(event Collision|EventActorBeginOverlap
  (params (OtherActor :type Actor%20Object%20Reference)))

(event EventTick
  (params (DeltaSeconds :type Float%20%28single-precision%29)))

(event EventToggle
  (bind _default_move (Variables|Default|Getdefault_move))
  (Audio|Components|Audio|Play _default_move 0.0)
  (if (Variables|Default|GetbOpen)
    (bind _angle (Timeline|Movement Reverse)
      (:Update
        (Transformation|SetRelativeRotation (Variables|Default|GetSM_Door01) (Math|Rotator|MakeRotator 0.0 0.0 (* _angle (Math|Float|SelectFloat -9e+01 9e+01 (Variables|Default|GetReverse)))) false false))
      (:Finished
        (Audio|Components|Audio|Stop _default_move)
        (Audio|PlaySoundatLocation (Variables|Default|GetFinishMovementSound) (Transformation|GetActorLocation) "0, 0, 0" 1.0 1.0 0.0 "/Game/SuperGrid/TutorialLevel/SoundEffects/Attenuation_Ambient.Attenuation_Ambient" 0 0)
        (Variables|Default|SetbOpen (not (Variables|Default|GetbOpen)))
        (Default|CallOnFinishedMovement)))
    (else
      (Timeline|Movement Play))))

(event EventUseItem
  (params (Item :type Actor%20Object%20Reference) (InteractedComponent :type Actor%20Component%20Object%20Reference))
  (|CallParentFunction Item InteractedComponent)
  (Development|PrintString (Utilities|GetDisplayName Item)))

(event EventOnUnlocked
  (Audio|PlaySoundatLocation (Variables|Default|GetDoorUnlockedSound) (Transformation|GetActorLocation) "0, 0, 0" 1.0 1.0 0.0 "/Game/SuperGrid/TutorialLevel/SoundEffects/Attenuation_Ambient.Attenuation_Ambient" 0 0))

(event EventPlayDoorLockedEffects
  (Audio|PlaySoundatLocation (Variables|Default|GetDoorLockedSound) (Transformation|GetActorLocation) "0, 0, 0" 1.0 1.0 0.0 "/Game/SuperGrid/TutorialLevel/SoundEffects/Attenuation_Ambient.Attenuation_Ambient" 0 0))

(fn ConstructionScript
  (Components|Timeline|SetPlayRate (Variables|Default|GetMovement) (Variables|Default|GetPlayRateOfTImeline)))

(fn ComponentstoSave
  (return 0))