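; BP_BreakableActor is a destructible actor that reacts to being broken and counts toward player tasks.
; When its Destructible component fractures, it turns off pickup on any HoldableActorComponent it has.
; It then reports its configured task name and amount to the player task manager and fires OnBroken.
; ComponentsToSave returns no components, and construction and tick add no logic.
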(event OnComponentFracture(Destructible)
  (params (HitPoint :type Vector%20%28by%20ref%29 :default "0, 0, 0") (HitDirection :type Vector%20%28by%20ref%29 :default "0, 0, 0"))
  (bind _returnvalue (Actor|GetComponentbyClass "/Script/Maintenance.HoldableActorComponent"))
  (Utilities|IsValid _returnvalue
    (:Is%20Valid
      (Variables|/Script/Maintenance.HoldableActorComponent|SetbCanBePickedUp _returnvalue false))
    (:Is%20Not%20Valid
      _))
  (Class|TaskInterface|OnTaskProgressed(Message) (CallFunction|GetPlayerTaskManager) (Utilities|Struct|MakeTask (Variables|Tasks|GetTaskName) "" 1) (Variables|Tasks|GetTaskAmount))
  (Default|CallOnBroken))

(event EventBeginPlay)

(event Collision|EventActorBeginOverlap
  (params (OtherActor :type Actor%20Object%20Reference)))

(event EventTick
  (params (DeltaSeconds :type Float%20%28single-precision%29)))

(fn ConstructionScript)

(fn ComponentstoSave
  (return 0))