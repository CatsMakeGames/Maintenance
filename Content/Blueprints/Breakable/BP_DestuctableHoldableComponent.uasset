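; Holdable component variant that lets breakable objects with destructible meshes be picked up, dropped and thrown.
; It handles the pickup, drop and throw events by looping over the owner's DestructibleComponents that carry the physics tag.
; Pickup turns off physics simulation on those components, drop turns it back on, and throw applies the given impulse to them.
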(event EventBeginPlay)

(event EventTick
  (params (DeltaSeconds :type Float%20%28single-precision%29)))

(event EventChildonbeDropped
  (for _array_element (Actor|GetComponentsByClass (Components|GetOwner) "/Script/ApexDestruction.DestructibleComponent")
    (if (!= (Utilities|Array|FindItem (Variables|/Script/Engine.ActorComponent|GetComponentTags _array_element) (Variables|Default|GetPhysComponentsTag)) -1)
      (Physics|SetSimulatePhysics _array_element true))))

(event EventChildonbePickedup
  (for _array_element (Actor|GetComponentsByClass (Components|GetOwner) "/Script/ApexDestruction.DestructibleComponent")
    (if (!= (Utilities|Array|FindItem (Variables|/Script/Engine.ActorComponent|GetComponentTags _array_element) (Variables|Default|GetPhysComponentsTag)) -1)
      (Physics|SetSimulatePhysics _array_element false))))

(event EventChildonThrown
  (params (impulse :type Vector :default "0, 0, 0"))
  (for _array_element (Actor|GetComponentsByClass (Components|GetOwner) "/Script/ApexDestruction.DestructibleComponent")
    (if (!= (Utilities|Array|FindItem (Variables|/Script/Engine.ActorComponent|GetComponentTags _array_element) (Variables|Default|GetPhysComponentsTag)) -1)
      (Physics|AddImpulse _array_element impulse "None" false))))