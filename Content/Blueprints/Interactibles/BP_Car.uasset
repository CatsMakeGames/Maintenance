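; Interactable car that accepts the car key and fuel tank as key items for intro tasks.
; UseKeys matches each supplied key's ID against CarKey, then FuelTank.
; A match completes a player task manager task and fires OnCarKeysUsed or OnFuelAdded.
; The task names are crossed: the car key completes "intro_CarFuel" and the fuel tank completes "intro_CarKeys".
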(event EventBeginPlay)

(event Collision|EventActorBeginOverlap
  (params (OtherActor :type Actor%20Object%20Reference)))

(event EventTick
  (params (DeltaSeconds :type Float%20%28single-precision%29)))

(event EventUseKeys
  (params (interactor :type Actor%20Object%20Reference) (Keys :type Array%20of%20Key%20Info%20Structures))
  (bind _manager (CallFunction|GetPlayerTaskManager))
  (for _array_element Keys
    (if (== (Utilities|Struct|BreakKeyInfo (Variables|/Script/Maintenance.KeyComponent|GetKeyInfo (Variables|Default|GetCarKey))) (.KeyId (Utilities|Struct|BreakKeyInfo _array_element)))
      (Class|TaskInterface|OnTaskCompleted(Message) _manager (Utilities|Struct|MakeTask "intro_CarFuel" "Get car fuel" 1))
      (Default|CallOnCarKeysUsed)
      (elif (== (Utilities|Struct|BreakKeyInfo (Variables|/Script/Maintenance.KeyComponent|GetKeyInfo (Variables|Default|GetFuelTank))) (.KeyId (Utilities|Struct|BreakKeyInfo _array_element)))
        (Class|TaskInterface|OnTaskCompleted(Message) _manager (Utilities|Struct|MakeTask "intro_CarKeys" "Get car keys" 1))
        (Default|CallOnFuelAdded)))))

(fn ConstructionScript)