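; Interactable story note that the player picks up in the world.
; The construction script fills Note from the DT_StoryNotes row selected by NoteData.
; On Interact it passes Note to BP_Player, plays a pickup sound, sets PickedUp, then hides itself and disables collision instead of being destroyed.
; ActorLoaded reapplies that hidden state if PickedUp is set, so collected notes stay gone after a load.
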(event EventBeginPlay)

(event Collision|EventActorBeginOverlap
  (params (OtherActor :type Actor%20Object%20Reference)))

(event EventTick
  (params (DeltaSeconds :type Float%20%28single-precision%29)))

(event EventInteract
  (params (Interactor :type Actor%20Object%20Reference) (InteractedComponent :type Actor%20Component%20Object%20Reference))
  (bind _asbp_player (Utilities|Casting|CastToBP_Player Interactor))
  (Class|MaintenanceCharacter|PickupNote _asbp_player (Variables|Internal|GetNote))
  (Audio|PlaySound2D "/Game/Sounds/Interact/PickItem0.PickItem0" 1.0 1.0 0.0 0 0)
  (Variables|SaveSystem|SetPickedUp true)
  (Rendering|SetActorHiddenInGame true)
  (Collision|SetActorEnableCollision false))

(event EventActorLoaded
  (if (Variables|SaveSystem|GetPickedUp)
    (Rendering|SetActorHiddenInGame true)
    (Collision|SetActorEnableCollision false)))

(fn ConstructionScript
  (bind _returnvalue (Utilities|GetDataTableRow "/Game/DataTables/DT_StoryNotes.DT_StoryNotes" (.RowName (Utilities|Struct|BreakDataTableRowHandle (Variables|Note|GetNoteData))))
    (:then
      (Variables|Internal|SetNote _returnvalue))))

(fn ComponentstoSave
  (return 0))