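; BP_Axe is a holdable axe tool that swings when used in hand and damages actors it touches mid-swing.
; Use plays the AxeMove timeline to pitch the mesh, with a Swinging flag blocking re-triggers until it finishes.
; Sphere overlaps during a swing apply generic damage, then a debug-drawn visibility trace toward the target applies additional point damage to whatever it hits.
; Pickup enables actor collision but disables the mesh's own.
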(event OnPickedUp(Holdable))

(event OnComponentBeginOverlap(Sphere)
  (params (OverlappedComponent :type Primitive%20Component%20Object%20Reference) (OtherActor :type Actor%20Object%20Reference) (OtherComp :type Primitive%20Component%20Object%20Reference) (OtherBodyIndex :type Integer) (bFromSweep :type Boolean) (SweepResult :type Hit%20Result%20Structure%20%28by%20ref%29))
  (if (Variables|Default|GetSwinging)
    (Game|Damage|ApplyDamage OtherActor 5e+01 0 0)
    (bind (_outhit _returnvalue) (Collision|LineTraceByChannel (Transformation|GetActorLocation) (Transformation|GetActorLocation OtherActor) "TraceTypeQuery1" false 0 "ForDuration"))
    (if _returnvalue
      (Game|Damage|ApplyPointDamage (.HitActor (Collision|BreakHitResult _outhit)) 5e+01 (.TraceStart (Collision|BreakHitResult _outhit)) _outhit))))

(event EventBeginPlay)

(event Collision|EventActorBeginOverlap
  (params (OtherActor :type Actor%20Object%20Reference)))

(event EventTick
  (params (DeltaSeconds :type Float%20%28single-precision%29)))

(event EventUseIteminHand
  (params (HoldingActor :type Actor%20Object%20Reference))
  (bind _sm_axe_01 (Variables|Default|GetSM_Axe_01))
  (if (not (Variables|Default|GetSwinging))
    (Variables|Default|SetSwinging true)
    (bind _axeswingrotation (Timeline|AxeMove PlayFromStart)
      (:Update
        (Transformation|SetRelativeRotation _sm_axe_01 (Math|Rotator|MakeRotator 0.0 _axeswingrotation 0.0) false false)
        (Transformation|SetRelativeLocation _sm_axe_01 "0, 0, 0" false false))
      (:Finished
        (Variables|Default|SetSwinging false)))))

(event EventOnToolPickedUp
  (Collision|SetActorEnableCollision true)
  (Collision|SetCollisionEnabled (Variables|Default|GetSM_Axe_01) "NoCollision"))

(fn ConstructionScript)