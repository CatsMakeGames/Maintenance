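; Player Blueprint that adds the inventory tool menu, jumpscare camera shake and task feedback on top of its parent class.
; An input action shows the menu, switching input mode and cursor, and task events play a diary sound or report completion.
; It saves its task component, restores held actors and tools on load, and reloads the level when caught.
; Numpad keys trigger saving and level reload.
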(event OnTaskfromListCompleted(TaskManagment)
  (params (task :type Task%20Structure))
  (Default|CallOnTaskCompleted (.Name (Utilities|Struct|BreakTask task))))

(event OnNewTaskAdded(TaskManagment)
  (Audio|PlaySound2D "/Game/HorrorEngine/Audio/SFX/DiaryUpdate.DiaryUpdate" 1.0 1.0 0.0 0 0))

(event Custom|PlayCameraJumspcareEffect
  (bind _asplayer_controller (Utilities|Casting|CastToPlayerController (Pawn|GetController)))
  (Class|PlayerController|ClientPlayCameraShake _asplayer_controller "/Game/Blueprints/CameraShakes/BP_JumpscareShake.BP_JumpscareShake_C" 1.0 "CameraLocal" "0, 0, 0"))

(event Custom|ShowToolMenuEvent
  (Input|SetInputModeUIOnly (Game|GetPlayerController 0) (Variables|Default|GetToolMenu) "DoNotLock")
  (CallFunction|SetShowMouse self true)
  (Widget|SetVisibility (Variables|Default|GetToolMenu) "Visible")
  (Default|OnBecomeVisible (Variables|Default|GetToolMenu)))

(event Custom|HideToolMenu
  (Input|SetInputModeGameOnly (Game|GetPlayerController 0))
  (CallFunction|SetShowMouse self false))

(event EventBeginPlay
  (|CallParentFunction)
  (bind _returnvalue (UserInterface|CreateWidget "/Game/Blueprints/UI/UMG_Invetory.UMG_Invetory_C" 0 self))
  (UserInterface|Viewport|AddtoViewport _returnvalue 0)
  (Variables|Default|SetToolMenu _returnvalue))

(event EventGetCaught
  (|CallParentFunction)
  (Utilities|FlowControl|Delay 1.0)
  (bind _returnvalue (Game|GetCurrentLevelName true))
  (Game|OpenLevel(byName) (Utilities|String|StringToName _returnvalue)))

(event EventActorLoaded
  (bind _currentlyheldactor (Variables|Default|GetCurrentlyHeldActor))
  ;[1 1 1] On load
  (Utilities|IsValid _currentlyheldactor
    (:Is%20Valid
      (Class|MaintenanceCharacter|ForcePickupActor _currentlyheldactor))
    (:Is%20Not%20Valid
      _))
  (Class|MaintenanceCharacter|ReattachTools))

(event Input|ActionEvents|InputActionShowToolMenu
  (params (Key :type Key%20Structure :default "None"))
  (:Pressed
    (Input|SetInputModeUIOnly (Game|GetPlayerController 0) (Variables|Default|GetToolMenu) "DoNotLock")
    (CallFunction|SetShowMouse self true)
    (Widget|SetVisibility (Variables|Default|GetToolMenu) "Visible")
    (Default|OnBecomeVisible (Variables|Default|GetToolMenu))))

(event Input|KeyboardEvents|Q
  (params (Key :type Key%20Structure :default "None")))

(event Input|KeyboardEvents|NumPadSeven
  (params (Key :type Key%20Structure :default "None"))
  (:Pressed
    (|AsyncSaveActors 3)))

(event Input|KeyboardEvents|NumPadEight
  (params (Key :type Key%20Structure :default "None"))
  (:Pressed
    (bind _returnvalue (Game|GetCurrentLevelName true))
    (Game|OpenLevel(byName) (Utilities|String|StringToName _returnvalue))))

(fn ConstructionScript)

(fn ComponentstoSave
  (return (Utilities|Array|MakeArray (Variables|Default|GetTaskManagment))))