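; Game mode that loads saved actor data when a player restarts and discards saves from a different game version.
; After a short delay, it runs an async full-reload actor load, then compares the local BP_SaveProfile's GameVersion against its own Version.
; On a mismatch or failed profile cast, it deletes all data for the current save slot and reopens the current level.
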(event EventBeginPlay)

(event EventTick
  (params (DeltaSeconds :type Float%20%28single-precision%29)))

(event EventOnRestartPlayer
  (params (NewPlayer :type Controller%20Object%20Reference))
  (Utilities|FlowControl|Delay 0.5)
  (|AsyncLoadActors 3 true
    (:OnCompleted
      (Development|PrintString "Loaded")
      (bind _asbp_save_profile (Utilities|Casting|CastToBP_SaveProfile (Class|EMSFunctionLibrary|GetLocalProfileSaveGame))
        (:then
          (if (Utilities|Enum|NotEqual(Enum) (Variables|/Game/Blueprints/SaveSystem/BP_SaveProfile.BP_SaveProfile_C|GetGameVersion _asbp_save_profile) (Variables|Default|GetVersion))
            (Class|EMSFunctionLibrary|DeleteAllSaveDataforSlot (.SaveGameName (Class|EMSFunctionLibrary|GetSlotInfoSaveGame)) :!label _label)
            (bind _returnvalue (Game|GetCurrentLevelName true))
            (Game|OpenLevel(byName) (Utilities|String|StringToName _returnvalue))))
        (:CastFailed
          (goto _label))))))

(fn ConstructionScript)