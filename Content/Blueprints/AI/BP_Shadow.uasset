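; Shadow enemy character that patrols and chases under a ShadowAIBase controller and catches the player on overlap.
; Seeing or losing the target switches walk speed and noise volume.
; A catch calls GetCaught, snaps the player's view to its head and plays an attack animation.
; Save hooks copy target, last seen and noise locations and patrol point from the controller, restoring them on load and spawning a controller if none exists.
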(event OnComponentBeginOverlap(PlayerCatchCollision)
  (params (OverlappedComponent :type Primitive%20Component%20Object%20Reference) (OtherActor :type Actor%20Object%20Reference) (OtherComp :type Primitive%20Component%20Object%20Reference) (OtherBodyIndex :type Integer) (bFromSweep :type Boolean) (SweepResult :type Hit%20Result%20Structure%20%28by%20ref%29))
  (bind _asbp_player (Utilities|Casting|CastToBP_Player OtherActor))
  (Audio|PlaySound2D (Variables|Default|GetGetCaughtSound) 1.0 1.0 0.0 0 0)
  (Class|MaintenanceCharacter|GetCaught _asbp_player)
  (bind _asplayer_controller (Utilities|Casting|CastToPlayerController (Pawn|GetController _asbp_player)))
  (Pawn|SetControlRotation _asplayer_controller (Math|Rotator|FindLookatRotation (Transformation|GetWorldLocation (Variables|/Script/Maintenance.MaintenanceCharacter|GetFirstPersonCameraComponent _asbp_player)) (Transformation|GetWorldLocation (Variables|Default|GetHeadPos))))
  (Transformation|AddRelativeLocation (Variables|Default|GetSpotLight) "0.000000,-100.000000, 0" false false)
  (Components|Animation|PlayAnimation (Variables|Character|GetMesh) "/Game/Scanned3DPeoplePack/Anims/Zombie/Zombie_Stand_To_Atk_1_IPC.Zombie_Stand_To_Atk_1_IPC" false))

(event EventBeginPlay
  (Variables|/Script/Engine.CharacterMovementComponent|SetMaxWalkSpeed (Variables|Character|GetCharacterMovement) (Variables|Speed|GetNormalSpeed))
  (bind _asshadow_aibase (Utilities|Casting|CastToShadowAIBase (Pawn|GetController)))
  (Class|ShadowAIBase|Setup _asshadow_aibase))

(event Collision|EventActorBeginOverlap
  (params (OtherActor :type Actor%20Object%20Reference)))

(event EventTick
  (params (DeltaSeconds :type Float%20%28single-precision%29)))

(event EventActorPreSave
  (bind _asshadow_aibase (Utilities|Casting|CastToShadowAIBase (Pawn|GetController)))
  (Variables|SaveSystem|SetTarget (Variables|/Script/Maintenance.ShadowAIBase|GetTarget _asshadow_aibase))
  (Variables|SaveSystem|SetLastSeenLocation (Variables|/Script/Maintenance.ShadowAIBase|GetLastSeenLocation _asshadow_aibase))
  (Variables|SaveSystem|SetLastNoiseLocation (Variables|/Script/Maintenance.ShadowAIBase|GetLastNoiseLocation _asshadow_aibase))
  (Variables|SaveSystem|SetPatrolPoint (Class|ShadowAIBase|GetCurrentPatrolPoint _asshadow_aibase)))

(event EventActorLoaded
  (bind _returnvalue (Pawn|GetController))
  (bind _asshadow_aibase (Utilities|Casting|CastToShadowAIBase _returnvalue)
    (:then
      (Class|ShadowAIBase|SetTarget _asshadow_aibase (Variables|SaveSystem|GetTarget))
      (Class|ShadowAIBase|SetLastSeenLocation _asshadow_aibase (Variables|SaveSystem|GetLastSeenLocation))
      (Class|ShadowAIBase|SetLastNoiseLocation _asshadow_aibase (Variables|SaveSystem|GetLastNoiseLocation))
      (Class|ShadowAIBase|SetPatrolLocation _asshadow_aibase (Variables|SaveSystem|GetPatrolPoint) (Variables|Default|GetPatrolPoints)))
    (:CastFailed
      (Utilities|IsValid _returnvalue
        (:Is%20Not%20Valid
          (bind _returnvalue_2 (Game|SpawnActorfromClass "/Game/Blueprints/AI/BP_ShadowController.BP_ShadowController_C" (Transformation|GetActorTransform) "AlwaysSpawn" 0 0))
          (Utilities|IsValid _returnvalue_2
            (:Is%20Valid
              (Pawn|Possess _returnvalue_2 self)
              (Class|ShadowAIBase|SetTarget _returnvalue_2 (Variables|SaveSystem|GetTarget))
              (Class|ShadowAIBase|SetLastSeenLocation _returnvalue_2 (Variables|SaveSystem|GetLastSeenLocation))
              (Class|ShadowAIBase|SetLastNoiseLocation _returnvalue_2 (Variables|SaveSystem|GetLastNoiseLocation))
              (Class|ShadowAIBase|SetPatrolLocation _returnvalue_2 (Variables|SaveSystem|GetPatrolPoint) (Variables|Default|GetPatrolPoints)))))))))

(event EventOnLostTarget
  (Variables|/Script/Engine.CharacterMovementComponent|SetMaxWalkSpeed (Variables|Character|GetCharacterMovement) (Variables|Speed|GetNormalSpeed))
  (Audio|Components|Audio|SetVolumeMultiplier (Variables|Default|Getnoise12) 0.01 :!class /Script/Engine.AudioComponent)
  (Development|PrintString "Lost"))

(event EventOnSawTarget
  (Variables|/Script/Engine.CharacterMovementComponent|SetMaxWalkSpeed (Variables|Character|GetCharacterMovement) (Variables|Speed|GetChaseSpeed))
  (Audio|Components|Audio|SetVolumeMultiplier (Variables|Default|Getnoise12) 1.0 :!class /Script/Engine.AudioComponent)
  (Development|PrintString "See"))

(fn ConstructionScript)

(fn CanbeSeen
  (return false))

(fn CanbeSeenbyThisShadow
  (params (Shadow :type Actor%20Object%20Reference) (SightRadius :type Float%20%28single-precision%29))
  (return false))

(fn ComponentstoSave
  (return 0))

(fn GetCurrentAIState
  (return "EAS_Normal"))

(fn GetPatrolPoints
  (return (Variables|Default|GetPatrolPoints)))