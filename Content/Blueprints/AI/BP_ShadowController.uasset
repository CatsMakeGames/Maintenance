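; BP_ShadowController is the AI controller for the Shadow, which runs the BT_Shadow behavior tree on BeginPlay.
; A looping one-second timer polls the AI Perception component for currently perceived sight and hearing actors and passes both lists to UpdatePerceivedActors.
; GetSightRadius simply returns the parent's value, and a node setting the player as the blackboard Target is left disconnected.
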(event Custom|Update
  (bind _aiperception (Variables|Default|GetAIPerception))
  (Class|ShadowAIBase|UpdatePerceivedActors (Class|AIPerceptionComponent|GetPerceivedActors _aiperception "/Script/AIModule.AISense_Sight") (Class|AIPerceptionComponent|GetPerceivedActors _aiperception "/Script/AIModule.AISense_Hearing")))

(event EventBeginPlay
  (|CallParentFunction)
  (AI|RunBehaviorTree "/Game/Blueprints/AI/BT_Shadow.BT_Shadow")
  (bind _returnvalue (Utilities|Time|SetTimerbyEvent (delegate Custom|Update) 1.0 true))
  (Variables|Default|SetUpdateTimerHandle _returnvalue))

(fn ConstructionScript)

(fn GetSightRadius
  (bind _returnvalue (|CallParentFunction))
  (return _returnvalue))