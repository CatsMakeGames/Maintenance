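; Zombie enemy Blueprint that catches the player and chops breakable dummies with an axe, driven by overlaps on its catch collision.
; Catching the player calls GetCaught, snaps their view to the zombie's head, shifts a spotlight and plays a sound and attack animation.
; For dummies, it halts movement during the axe montage, applies delayed point damage using a line trace, then restores speed on completion.
; Save and load events only print debug messages.
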(event OnComponentBeginOverlap(PlayerCatchCollision)
  (params (OverlappedComponent :type Primitive%20Component%20Object%20Reference) (OtherActor :type Actor%20Object%20Reference) (OtherComp :type Primitive%20Component%20Object%20Reference) (OtherBodyIndex :type Integer) (bFromSweep :type Boolean) (SweepResult :type Hit%20Result%20Structure%20%28by%20ref%29))
  (bind _sm_axe_01 (Variables|Default|GetSM_Axe_01))
  (bind _returnvalue (Transformation|GetWorldLocation _sm_axe_01))
  (bind _asbp_player (Utilities|Casting|CastToBP_Player OtherActor)
    (:then
      (Audio|PlaySound2D (Variables|Default|GetGetCaughtSound) 1.0 1.0 0.0 0 0)
      (Class|MaintenanceCharacter|GetCaught _asbp_player)
      (bind _asplayer_controller (Utilities|Casting|CastToPlayerController (Pawn|GetController _asbp_player)))
      (Pawn|SetControlRotation _asplayer_controller (Math|Rotator|FindLookatRotation (Transformation|GetWorldLocation (Variables|/Script/Maintenance.MaintenanceCharacter|GetFirstPersonCameraComponent _asbp_player)) (Transformation|GetWorldLocation (Variables|Default|GetHeadPos))))
      (Transformation|AddRelativeLocation (Variables|Default|GetSpotLight) "0.000000,-100.000000, 0" false false)
      (Components|Animation|PlayAnimation (Variables|Character|GetMesh) "/Game/Scanned3DPeoplePack/Anims/Zombie/Zombie_Stand_To_Atk_1_IPC.Zombie_Stand_To_Atk_1_IPC" false))
    (:CastFailed
      (bind _asbp_breakable_dummy_base (Utilities|Casting|CastToBP_BreakableDummyBase OtherActor))
      (Animation|Montage|PlayMontage (Variables|Character|GetMesh) "/Game/Scanned3DPeoplePack/Anims/Generic/Anim_UseAxe_Montage.Anim_UseAxe_Montage"
        (:then
          (Variables|/Script/Engine.CharacterMovementComponent|SetMaxWalkSpeed (Variables|Character|GetCharacterMovement) 0.0)
          (Utilities|FlowControl|Delay 1.2)
          (bind _outhit (Collision|LineTraceByChannel _returnvalue (Transformation|GetActorLocation _asbp_breakable_dummy_base) "TraceTypeQuery1" false 0 "None"))
          (Game|Damage|ApplyPointDamage _asbp_breakable_dummy_base 1e+02 _returnvalue _outhit))
        (:OnCompleted
          (Variables|/Script/Engine.CharacterMovementComponent|SetMaxWalkSpeed (Variables|Character|GetCharacterMovement) (Variables|Default|GetCurrentSpeed)))))))

(event EventBeginPlay
  (|CallParentFunction))

(event Collision|EventActorBeginOverlap
  (params (OtherActor :type Actor%20Object%20Reference))
  (|CallParentFunction OtherActor) ; This node is disabled and will not be called.\nDrag off pins to build functionality.
)

(event EventTick
  (params (DeltaSeconds :type Float%20%28single-precision%29))
  (|CallParentFunction DeltaSeconds) ; This node is disabled and will not be called.\nDrag off pins to build functionality.
)

(event EventActorLoaded
  (|CallParentFunction)
  (Development|PrintString "Zombie man loaded"))

(event EventActorSaved
  (Development|PrintString "Zombie man saved" true true "(R=1.000000,G=0.000000,B=0.414306,A=1.000000)"))

(fn ConstructionScript
  (|CallParentFunction))