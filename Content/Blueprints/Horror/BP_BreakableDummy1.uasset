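; BP_BreakableDummy1 is a breakable dummy prop in the Horror folder that can randomly appear.
; Appear checks CanAppear and a weighted chance, then unhides the destructible mesh, enables blocking collision and clears CanDissapear.
; It also sets Visible to false despite showing the mesh.
; The mesh's fracture event sets Destroyed; nothing in this Blueprint calls Appear or reads that flag.
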(event OnComponentFracture(SM_Dummy_Idle3_DM)
  (params (HitPoint :type Vector%20%28by%20ref%29 :default "0, 0, 0") (HitDirection :type Vector%20%28by%20ref%29 :default "0, 0, 0"))
  (Variables|Default|SetDestroyed true))

(event EventBeginPlay)

(fn ConstructionScript)

(fn Appear
  (bind _sm_dummy_idle3_dm (Variables|Default|GetSM_Dummy_Idle3_DM))
  (if (Variables|Default|GetCanAppear)
    (if (Math|Random|RandomBoolwithWeight (Variables|Default|GetChanceOfAppearing))
      (Variables|Default|SetVisible false)
      (Development|SetHiddeninGame _sm_dummy_idle3_dm false false)
      (Collision|SetCollisionEnabled _sm_dummy_idle3_dm "QueryAndPhysics")
      (Variables|Default|SetCanDissapear false)
      (Collision|SetCollisionResponsetoAllChannels _sm_dummy_idle3_dm "ECR_Block"))))