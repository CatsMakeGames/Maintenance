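; BP_ShadowOfOldLife is a horror scare actor with skeletal mesh figures, triggered when the player enters its box.
; After a short delay, it plays the player's camera jumpscare effect and a 2D horror sound.
; It then switches RadioMusic to a radio tuning sound and hides all of its skeletal mesh components.
; The overlap has no one-shot guard, and the box is never disabled here.
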(event OnComponentBeginOverlap(Box)
  (params (OverlappedComponent :type Primitive%20Component%20Object%20Reference) (OtherActor :type Actor%20Object%20Reference) (OtherComp :type Primitive%20Component%20Object%20Reference) (OtherBodyIndex :type Integer) (bFromSweep :type Boolean) (SweepResult :type Hit%20Result%20Structure%20%28by%20ref%29))
  (bind _asbp_player (Utilities|Casting|CastToBP_Player OtherActor))
  (Utilities|FlowControl|Delay 3.0)
  (Default|PlayCameraJumspcareEffect _asbp_player)
  (Audio|PlaySound2D "/Game/Sounds/Horror/Horror11.Horror11" 1.0 1.0 0.0 0 0)
  (Audio|Components|Audio|SetSound (Variables|Default|GetRadioMusic) "/Game/HorrorEngine/Audio/Radio/RadioTuning01.RadioTuning01")
  (for _array_element (Actor|GetComponentsByClass "/Script/Engine.SkeletalMeshComponent")
    (Development|SetHiddeninGame _array_element true false)))

(event EventBeginPlay)

(event Collision|EventActorBeginOverlap
  (params (OtherActor :type Actor%20Object%20Reference)))

(event EventTick
  (params (DeltaSeconds :type Float%20%28single-precision%29)))

(fn ConstructionScript)

(fn ComponentstoSave
  (return 0))