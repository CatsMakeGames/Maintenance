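; Horror scare actor: a shadow that faces its Target while unseen and serves as a one-shot jumpscare.
; Tick uses render-recency checks to rotate it toward the Target only while off-screen, as long as Moved is false.
; With Moved true, being rendered plays a 2D spook sound, destroys the actor and triggers the Target's camera jumpscare effect.
; Moved is never set here, and the teleport to the Target's BehindLocation is disconnected.
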(event EventBeginPlay)

(event Collision|EventActorBeginOverlap
  (params (OtherActor :type Actor%20Object%20Reference)))

(event EventTick
  (params (DeltaSeconds :type Float%20%28single-precision%29))
  (bind _target (Variables|Default|GetTarget))
  (Utilities|IsValid _target
    (:Is%20Valid
      (if (Variables|Default|GetMoved)
        (if (Class|Actor|WasRecentlyRendered 0.05)
          (Audio|PlaySound2D (Variables|Default|GetSpookSound) 1.0 1.0 0.0 0 0)
          (Actor|DestroyActor)
          (Default|PlayCameraJumspcareEffect (Variables|Default|GetTarget)))
        (elif (not (Class|Actor|WasRecentlyRendered 0.1))
          (Transformation|SetActorRotation (Math|Rotator|FindLookatRotation (Transformation|GetActorLocation) (Transformation|GetActorLocation _target))))))))

(fn ConstructionScript)