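; One-shot horror scare actor in which a skeletal mesh figure runs by when the player enters a trigger box.
; The first BP_Player overlap sets the Spooked flag, plays a 2D spook sound and starts the RunBy timeline.
; The timeline slides the mesh along its relative Y axis, scaling its Amount track by the Distance variable, without sweeping.
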(event OnComponentBeginOverlap(Box)
  (params (OverlappedComponent :type Primitive%20Component%20Object%20Reference) (OtherActor :type Actor%20Object%20Reference) (OtherComp :type Primitive%20Component%20Object%20Reference) (OtherBodyIndex :type Integer) (bFromSweep :type Boolean) (SweepResult :type Hit%20Result%20Structure%20%28by%20ref%29))
  (if (not (Variables|Default|GetSpooked))
    (Utilities|Casting|CastToBP_Player OtherActor)
    (Variables|Default|SetSpooked true)
    (Audio|PlaySound2D (Variables|Default|GetSpookSound) 1.0 1.0 0.0 0 0)
    (bind _amount (Timeline|RunBy PlayFromStart)
      (:Update
        (Transformation|SetRelativeLocation (Variables|Default|GetSkeletalMesh) (Math|Vector|MakeVector 0.0 (* _amount (Variables|Default|GetDistance)) 0.0) false false)))))

(event EventBeginPlay)

(event Collision|EventActorBeginOverlap
  (params (OtherActor :type Actor%20Object%20Reference)))

(event EventTick
  (params (DeltaSeconds :type Float%20%28single-precision%29)))

(fn ConstructionScript)

(fn ComponentstoSave
  (return 0))