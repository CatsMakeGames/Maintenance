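; BP_SpookySlidingDoor is a horror sliding door that can suddenly open or freak out when its functions are called.
; SuddenlyOpen plays an opening sound and a timeline that slides the Door along local Y, with another sound when it finishes.
; StartFreakingOut plays one of three BrokenDoor timelines at random, each moving the door the same way and triggering slide sounds through event tracks.
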(event EventBeginPlay)

(event Collision|EventActorBeginOverlap
  (params (OtherActor :type Actor%20Object%20Reference)))

(event EventTick
  (params (DeltaSeconds :type Float%20%28single-precision%29)))

(fn ConstructionScript)

(fn SuddenlyOpen
  (Audio|Components|Audio|Play (Variables|Default|Getdoorslide_opening1) 0.0)
  (Audio|Components|Audio|Play (Variables|Default|GetSuddenlyOpen_Timeline)))

(fn StartFreakingOut
  (Audio|Components|Audio|Play (Utilities|Select :Index (Math|Random|RandomIntegerinRange 0 2) :Option%200 (Variables|Default|GetBrokenDoor) :Option%201 (Variables|Default|GetBrokenDoor1) :Option%202 (Variables|Default|GetBrokenDoor2))))