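; BP_Dummy is a horror mannequin that vanishes when out of view, after it has been seen.
; Tick arms disappearance once the actor was recently rendered, then hides the mesh and sets its collision to overlap when rendering stops.
; Appear rolls a weighted chance, if allowed, to show it with blocking collision and reset that arming.
; Mesh overlap only prints a debug string.
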(event OnComponentBeginOverlap(UE4_Mannequin)
  (params (OverlappedComponent :type Primitive%20Component%20Object%20Reference) (OtherActor :type Actor%20Object%20Reference) (OtherComp :type Primitive%20Component%20Object%20Reference) (OtherBodyIndex :type Integer) (bFromSweep :type Boolean) (SweepResult :type Hit%20Result%20Structure%20%28by%20ref%29))
  (Development|PrintString "I can show "))

(event EventBeginPlay)

(event Collision|EventActorBeginOverlap
  (params (OtherActor :type Actor%20Object%20Reference)))

(event EventTick
  (params (DeltaSeconds :type Float%20%28single-precision%29))
  (if (Variables|Default|GetCanDissapear)
    (if (not (Class|Actor|WasRecentlyRendered 0.01))
      (Variables|Default|SetVisible false)
      (Rendering|SetVisibility (Variables|Default|GetUE4_Mannequin) false false)
      (Collision|SetCollisionResponsetoAllChannels (Variables|Default|GetUE4_Mannequin) "ECR_Overlap"))
    (elif (Class|Actor|WasRecentlyRendered 0.2)
      (Variables|Default|SetCanDissapear true))))

(fn ConstructionScript)

(fn Appear
  (if (Variables|Default|GetCanAppear)
    (if (Math|Random|RandomBoolwithWeight (Variables|Default|GetChanceOfAppearing))
      (Variables|Default|SetVisible true)
      (Rendering|SetVisibility (Variables|Default|GetUE4_Mannequin) true false)
      (Collision|SetCollisionResponsetoAllChannels (Variables|Default|GetUE4_Mannequin) "ECR_Block")
      (Variables|Default|SetCanDissapear false))))